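; Guide arrow for an educational AR tour that floats ahead of the camera and points toward the current project stop.
; Tick keeps its text facing the camera and hides arrow and text near any of the three project text actors.
; Reaching the target shows an info popup for that project and cycles the target to the next.
; BeginPlay adds a pause button and sets Dutch or English copy from the saved language ID.
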(event `self.ReceiveBeginPlay`
  (`self.setLanguage`)
  (bind _returnvalue (`|CreateWidget` "/Game/UI/PauseButton.PauseButton_C"))
  (`UserWidget.AddToViewport` _returnvalue 0))

(event `self.ReceiveTick`
  (params (DeltaSeconds :type "Float (single-precision)"))
  (bind _returnvalue (`GameplayStatics.GetPlayerCameraManager` 0))
  (bind _currentproject (`self.currentProject`))
  (bind _returnvalue_2 (`PlayerCameraManager.GetCameraLocation` _returnvalue))
  (bind _returnvalue_3 (- (`self.location`) (`self.K2_GetActorLocation`)))
  (`self.rotateText`)
  (`self.K2_SetActorLocationAndRotation` (`KismetMathLibrary.MakeVector` (.x (`KismetMathLibrary.TransformLocation` (`KismetMathLibrary.Conv_VectorToTransform` _returnvalue_2) (* (`self.GetActorForwardVector` _returnvalue) (300.0 300.0 0.0)))) (.y (`KismetMathLibrary.TransformLocation` (`KismetMathLibrary.Conv_VectorToTransform` _returnvalue_2) (* (`self.GetActorForwardVector` _returnvalue) (300.0 300.0 0.0)))) -175.0) (`KismetMathLibrary.MakeRotator` 0.0 20.0 (.yaw (`KismetMathLibrary.MakeRotFromXY` _returnvalue_3 _returnvalue_3))))
  (`|ExecutionSequence`
    (:`then_0`
      (bind _returnvalue_4 (`GameplayStatics.GetActorOfClass` "/Game/WebDevelopment/WebDevText.WebDevText_C"))
      (bind _returnvalue_5 (`GameplayStatics.GetActorOfClass` "/Game/Database/DatabaseText.DatabaseText_C"))
      (bind _returnvalue_6 (`GameplayStatics.GetActorOfClass` "/Game/Battlebot/BattleBotText.BattleBotText_C"))
      (bind _returnvalue_7 (not (or (< (`KismetMathLibrary.VSize` (- (`self.K2_GetActorLocation` _returnvalue_4) _returnvalue_2)) (`self.distanceToHide`)) (< (`KismetMathLibrary.VSize` (- (`self.K2_GetActorLocation` _returnvalue_5) _returnvalue_2)) (`self.distanceToHide`)) (< (`KismetMathLibrary.VSize` (- (`self.K2_GetActorLocation` _returnvalue_6) _returnvalue_2)) (`self.distanceToHide`)))))
      (`SceneComponent.SetVisibility` (`self.ArrowEduArTour`) _returnvalue_7 false)
      (`SceneComponent.SetVisibility` (`self.Text`) _returnvalue_7 false))
    (:`then_1`
      (if (not (>= (`KismetMathLibrary.VSize` (- (`self.location`) _returnvalue_2)) (`self.distanceToHide`)))
        (if (> _currentproject 2)
          (set `self.currentProject` 0)
          (else
            (set `self.currentProject` (+ _currentproject 1))))
        (switch `int` (`self.currentProject`)
          (:`0`
            (bind _returnvalue_8 (`GameplayStatics.GetActorOfClass` "/Game/WebDevelopment/WebDevText.WebDevText_C"))
            (set `self.location` (`self.K2_GetActorLocation` _returnvalue_8))
            (`WidgetLayoutLibrary.RemoveAllWidgets`)
            (bind _returnvalue_9 (`|CreateWidget` "/Game/BP_InfoPopUp.BP_InfoPopUp_C"))
            (`UserWidget.AddToViewport` _returnvalue_9 0)
            (`/Game/BP_InfoPopUp.SetContent` _returnvalue_9 "BattleBot" (`KismetTextLibrary.Conv_TextToString` (`self.BattleBotText`))))
          (:`1`
            (bind _returnvalue_10 (`GameplayStatics.GetActorOfClass` "/Game/Database/DatabaseText.DatabaseText_C"))
            (set `self.location` (`self.K2_GetActorLocation` _returnvalue_10))
            (`WidgetLayoutLibrary.RemoveAllWidgets`)
            (bind _returnvalue_11 (`|CreateWidget` "/Game/BP_InfoPopUp.BP_InfoPopUp_C"))
            (`UserWidget.AddToViewport` _returnvalue_11 0)
            (`/Game/BP_InfoPopUp.SetContent` _returnvalue_11 "Web Development" (`KismetTextLibrary.Conv_TextToString` (`self.WebDevText`))))
          (:`2`
            (bind _returnvalue_12 (`GameplayStatics.GetActorOfClass` "/Game/Battlebot/BattleBotText.BattleBotText_C"))
            (set `self.location` (`self.K2_GetActorLocation` _returnvalue_12))
            (`WidgetLayoutLibrary.RemoveAllWidgets`)
            (bind _returnvalue_13 (`|CreateWidget` "/Game/BP_InfoPopUp.BP_InfoPopUp_C"))
            (`UserWidget.AddToViewport` _returnvalue_13 0)
            (`/Game/BP_InfoPopUp.SetContent` _returnvalue_13 "Database" (`KismetTextLibrary.Conv_TextToString` (`self.DatabaseText`)))))))))

(fn `rotateText`
  (`SceneComponent.K2_SetWorldRotation` (`self.Text`) (`KismetMathLibrary.FindLookAtRotation` (`SceneComponent.K2_GetComponentLocation` (`self.Text`)) (`PlayerCameraManager.GetCameraLocation` (`GameplayStatics.GetPlayerCameraManager` 0))) false false))

(fn `setLanguage`
  (bind _returnvalue (`GameplayStatics.LoadGameFromSlot` "LanguageID"))
  (bind _assave_game (cast `/Game/SaveGame` _returnvalue)
    (:`then`
      (bind _languageid (`/Game/SaveGame.getLanguageID` _assave_game))
      (if (== _languageid 0)
        (set `self.WebDevText` "In de eerste periode van het studiejaar is de opdracht gegeven om een project te ontwerpen en realiseren. Bij het project Web Development en Design is het de bedoeling om een (professionele) website voor een interne opdrachtgever te bouwen. Deze opdrachtgever heeft een bepaalde doelstelling die hij/zij/hen wil bereiken door middel van de ontworpen website. Het is aan de projectgroep om deze doelstelling mee te nemen in het ontwerpproces en de uiteindelijke realisatie van het product (website). De website wordt geprogrammeerd met Visual Studio Code in HTML en CSS. ")
        (set `self.DatabaseText` "Databases zijn programma’s die gegevens opslaan en beschikbaar maken. Veel programma’s maken gebruik van databases. Je maakt zelf waarschijnlijk dagelijks gebruik van databases. Als je geld opneemt bij de pinautomaat raadpleeg je de database van de bank. Als je een nieuw paspoort aanvraagt, wordt er ongetwijfeld een database met persoonsgegevens geraadpleegd. Databases vormen eigenlijk de basis van ieder informatiesysteem.  \n \nIn de tweede periode van het studiejaar is de opdracht gegeven om een database te ontwerpen en toe te passen voor een interne opdrachtgever. Dit wordt (deels) geprogrammeerd in de programmeertaal PHP. Naast het ontwerpen van een database leer je de gegevens in de database te raadplegen door middel van SQL. ")
        (set `self.BattleBotText` "1.	Klik één keer: De BattleBot begint te zweven. \n2.	Klik opnieuw: De BattleBot rijdt verder. \n3.	Houd vast: De BattleBot explodeert. \n4.	Sleep de BattleBot: De BattleBot roteert.  \nGebruik deze eenvoudige stappen om je BattleBot te bedienen! \n \nArduino is een populair platform voor het bouwen van elektrische projecten. Het bestaat uit hardware (microcontrollers) en software (Arduino IDE). De hardware is een kleine computer die je kunt programmeren om verschillende taken uit te voeren. De software gebruik je om die programma’s te schrijven en naar de microcontroller te uploaden.  \n \nIn de derde periode van het studiejaar is de opdracht gegeven om een Arduino Nano robot te programmeren. Arduino Nano is een specifieke versie van de Arduino microcontrollers. Het is klein van formaat, maar heeft genoeg kracht om allerlei taken uit te voeren. Dit wordt gedaan met Arduino IDE (Integrated Development Environment) in de programmeertalen C/C++. Het doel is om de ‘BattleBot’ correct aan te sluiten en te programmeren, zodat het in staat is om volledig zelfstandig en zo snel mogelijk in estafettevorm een parcours met obstakels af te leggen. Er zijn drie onderdelen: lijn volgen, lijn doolhof en fysiek doolhof.  ")
        (`TextRenderComponent.K2_SetText` (`self.Text`) (`KismetTextLibrary.Conv_StringToText` "Volg de pijl"))
        (else
          (set `self.WebDevText` "In the first period of the academic year, we were tasked with designing and implementing a project. For the Web Development and Design project, the goal is to build a (professional) website for an internal client. This client has specific objectives they want to achieve through the designed website. It is up to the project group to incorporate these objectives into the design process and the final product (website). The website will be programmed using Visual Studio Code in HTML and CSS. " :!label _label)
          (set `self.DatabaseText` "Databases are programs that store and provide access to data. Many applications use databases, and you probably interact with databases daily. For example, when you withdraw money from an ATM, you access the bank's database. When you apply for a new passport, a database of personal information is consulted. Databases are essentially the foundation of any information system.  \n \nIn the second period of the academic year, we were tasked with designing and implementing a database for an internal client. This will be partially programmed in the PHP programming language. In addition to designing a database, you will learn to query data in the database using SQL. ")
          (set `self.BattleBotText` "1.	Click once: The BattleBot starts to hover. \n2.	Click again: The BattleBot continues driving. \n3.	Hold: The BattleBot explodes. \n4.	Drag the BattleBot: The BattleBot rotates. \nUse this simple steps to control your BattleBot! \n \nArduino is a popular platform for building electronic projects. It consists of hardware (microcontrollers) and software (Arduino IDE). The hardware is a small computer that can be programmed to perform various tasks. The software is used to write these programs and upload them to the microcontroller.  \n \nIn the third period of the academic year, we were tasked with programming an Arduino Nano robot. The Arduino Nano is a specific version of the Arduino microcontrollers. It is small in size but powerful enough to perform various tasks. This will be done using the Arduino IDE (Integrated Development Environment) in the C/C++ programming languages. The goal is to correctly connect and program the 'BattleBot' so that it can autonomously and as quickly as possible complete an obstacle course in relay form. There are three components: line following, line maze, and physical maze. ")
          (`TextRenderComponent.K2_SetText` (`self.Text`) (`KismetTextLibrary.Conv_StringToText` "Follow the arrow")))))
    (:`CastFailed`
      (goto _label))))

(fn `UserConstructionScript`)