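; Touch input Blueprint that lets the player tap, hold and drag a Battlebot to change its state or spin it.
; On press it traces under the finger for a tagged Battlebot; movement beyond a small threshold cancels tap and hold.
; A tap toggles Driving and Hovering or turns Exploding to Hovering; a hold, timed on Tick, enters Exploding or returns to Driving.
; Horizontal drags spin the bot while Exploding.
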(event `InputTouch`
  (params (Location :type "Vector Structure") (FingerIndex :type "ETouchIndex Enum"))
  (bind _x (.x Location))
  (bind _battlebot (`self.battlebot`))
  (:`Pressed`
    ;[1 1 1] Grab Battlebot
    (bind _asplayer_controller (cast `PlayerController` (`GameplayStatics.GetPlayerController` 0)))
    (bind (_hitresult _returnvalue) (`self.GetHitResultUnderFingerForObjects` _asplayer_controller "Touch1" (`|MakeArray` "ObjectTypeQuery2" :!type "EObjectTypeQuery Enum") false))
    (if _returnvalue
      (bind (_bblockinghit _binitialoverlap _time _distance _location _impactpoint _normal _impactnormal _physmat _hitactor) (`GameplayStatics.BreakHitResult` _hitresult))
      (if (`self.ActorHasTag` _hitactor "Battlebot")
        (set `self.battlebot` _hitactor)
        (set `self.firstRun` true)
        (set `self.isPressed` true)
        (set `self.isMoved` false)
        (set `self.startLoc` Location)
        (else
          (set `self.battlebot` null :!label _label)))
      (else
        (goto _label))))
  (:`Released`
    (if (`self.isPressed`)
      (if (`KismetSystemLibrary.IsValid` (`self.battlebot`)) :!label _label_2
        (`|ExecutionSequence`
          (:`then_0`
            (if (not (`self.isMoved`))
              (bind _asbattlebot (cast `/Game/Battlebot/Blueprints/Battlebot` (`self.battlebot`)))
              (if (< (`self.heldTimer`) (`self.timeToHold`))
                (bind _battlebotstate (`/Game/Battlebot/Blueprints/Battlebot.battlebotState` _asbattlebot))
                (switch `/Game/Battlebot/Blueprints/BattlebotState` _battlebotstate ; This is called when the battlebot is pressed
                  (:`NewEnumerator0`
                    (set `/Game/Battlebot/Blueprints/Battlebot.battlebotState` "NewEnumerator1" _asbattlebot :!label _label_3))
                  (:`NewEnumerator1`
                    (set `/Game/Battlebot/Blueprints/Battlebot.battlebotState` "NewEnumerator0" _asbattlebot :!label _label_4))
                  (:`NewEnumerator2`
                    (goto _label_3)))
                (else
                  (switch `/Game/Battlebot/Blueprints/BattlebotState` _battlebotstate ; This is called when the battlebot is held
                    (:`NewEnumerator0`
                      _)
                    (:`NewEnumerator1`
                      _)
                    (:`NewEnumerator2`
                      (goto _label_4)))
                  (set `/Game/Battlebot/Blueprints/Battlebot.battlebotState` "NewEnumerator2" _asbattlebot)))))
          (:`then_1`
            (set `self.heldTimer` 0.0)
            (set `self.battlebot` null)
            (set `self.isPressed` false))))))
  (:`Moved`
    (`|ExecutionSequence`
      (:`then_0`
        (if (not (`self.isMoved`))
          (set `self.isMoved` (> (`KismetMathLibrary.Vector_Distance2D` (`self.startLoc`) Location) 20.0))))
      (:`then_1`
        ;[1 1 1] Drag Battlebot
        (if (`KismetSystemLibrary.IsValid` _battlebot)
          (bind _asbattlebot_2 (cast `/Game/Battlebot/Blueprints/Battlebot` _battlebot))
          (switch `/Game/Battlebot/Blueprints/BattlebotState` (`/Game/Battlebot/Blueprints/Battlebot.battlebotState` _asbattlebot_2)
            (:`NewEnumerator2`
              (if (`self.firstRun`)
                (set `self.lastX` _x)
                (set `self.firstRun` false)
                (else
                  (bind _asbattlebot_3 (cast `/Game/Battlebot/Blueprints/Battlebot` _battlebot))
                  (bind _result (`/Engine/EditorBlueprintResources/StandardMacros.NegateFloat` (* (`self.rotationSpeed`) (- _x (`self.lastX`))))
                    (:`  `
                      (`/Game/Battlebot/Blueprints/Battlebot.Spin` _asbattlebot_3 _result)
                      (set `self.lastX` _x))))))))))))

(event `self.ReceiveTick`
  (params (DeltaSeconds :type "Float (single-precision)"))
  (if (`self.isMoved`)
    _
    (elif (`self.isPressed`)
      (bind _output_get (set `self.heldTimer` (+ (`self.heldTimer`) DeltaSeconds)))
      (if (> _output_get (`self.timeToHold`))
        (goto _label_2)))))

(fn `UserConstructionScript`)