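; Battlebot display actor that switches between driving along a selected spline path, hovering while rotating, and an exploded component view.
; Tick detects state changes, saves the previous Driving or Hovering pose, then lerps the mesh to the new one before running that state's loop.
; Driving spins wheels and follows the spline by timeline, Hovering bobs on a sine wave, and Exploding pushes components along preset vectors, lerped back afterward.
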(event `StateSwap`
  (bind _returnvalue (`SceneComponent.GetRelativeTransform` (`self.BattleBot Mesh`)))
  (bind (_returnvalue_location _returnvalue_rotation _returnvalue_scale) (`KismetMathLibrary.BreakTransform` (`SceneComponent.GetRelativeTransform` (`self.BattleBot Mesh`))))
  ;[1 0.2029 0.1979] State Swap - Handles all functionality that happens upon the battlebots' state swapping, runs once per swap
  (`self.Reset State`)
  (set `self.moveToStart` (`SceneComponent.GetRelativeTransform` (`self.BattleBot Mesh`)))
  (`|ExecutionSequence`
    (:`then_0`
      (switch `/Game/Battlebot/Blueprints/BattlebotState` (`self.prevBattlebotState`)
        (:`NewEnumerator0`
          (set `self.LastPositionDriving` _returnvalue))
        (:`NewEnumerator1`
          (set `self.LastPositionHovering` _returnvalue))))
    (:`then_1`
      (set `self.moveToDelta` 0.0)
      (switch `/Game/Battlebot/Blueprints/BattlebotState` (`self.battlebotState`)
        (:`NewEnumerator0`
          (set `self.moveToEnd` (`self.LastPositionDriving`)))
        (:`NewEnumerator1`
          (set `self.moveToEnd` (`self.LastPositionHovering`))
          (if (== (`self.degrees`) 270.0)
            (set `self.moveToDelta` 2.0 :!label _label)))
        (:`NewEnumerator2`
          (set `self.moveToEnd` (`KismetMathLibrary.MakeTransform` (+ _returnvalue_location (0.0 0.0 500.0)) _returnvalue_rotation _returnvalue_scale)))))
    (:`then_2`
      (if (== (`KismetMathLibrary.MakeTransform` (0.0 0.0 0.0)) (`self.moveToEnd`))
        (goto _label)))))

(event `ResetExplode`
  ;[1 0.2029 0.1979] Reset Explode - Sets the variables used in the reset loop
  (set `self.unexplodeDistanceLeft` 100.0) ; To make sure the loop runs
  (set `self.unexplodeDelta` 0.0)
  (`KismetArrayLibrary.Array_Clear` (`self.endVector`))
  (for _array_element (`self.explodeComponents`)
    (`KismetArrayLibrary.Array_Add` (`self.endVector`) (`SceneComponent.RelativeLocation` _array_element))))

(event `self.ReceiveBeginPlay`
  ;[1 1 1] Setup
  (set `self.wheels` (`|MakeArray` (`self.LeftWheel`) (`self.RightWheel`)))
  (bind _output_get (set `self.explodeComponents` (`|MakeArray` (`self.Arduino`) (`self.LeftWheel`) (`self.RightWheel`) (`self.EchoSensor`) (`self.Powerbank`) (`self.IRSensor`) (`self.Gripper`) (`self.FrontWheel`))))
  (for _array_element _output_get
    (`KismetArrayLibrary.Array_Add` (`self.baseVectors`) (`SceneComponent.RelativeLocation` _array_element)))
  (set `self.moveVectors` (`|MakeArray` (0.0 0.0 -1.0) (-0.5 0.5 0.0) (-0.5 -0.5 0.0) (1.0 0.0 0.0) (0.0 0.0 -0.5) (0.25 0.0 0.5) (0.5 0.0 0.25) (0.0 0.0 0.75) :!type "Vector Structure"))
  (switch `/Game/Battlebot/Blueprints/SelectedPath` (`self.Selected Path`)
    (:`NewEnumerator0`
      (bind _returnvalue (`GameplayStatics.GetActorOfClass` "/Game/Battlebot/Blueprints/BP_SplinePath.BP_SplinePath_C"))
      (set `self.Road` (`/Game/Battlebot/Blueprints/BP_SplinePath.Road` _returnvalue)))
    (:`NewEnumerator1`
      (bind _returnvalue_2 (`GameplayStatics.GetActorOfClass` "/Game/Battlebot/Blueprints/BP_SplineMaze.BP_SplineMaze_C"))
      (set `self.Road` (`/Game/Battlebot/Blueprints/BP_SplineMaze.Spline` _returnvalue_2)))
    (:`NewEnumerator2`
      (`GameplayStatics.GetActorOfClass` null))))

(event `ResetExplodeLoop`
  (bind _returnvalue (+ (* (`GameplayStatics.GetWorldDeltaSeconds`) 0.1) (`self.unexplodeDelta`)))
  ;[1 0.2039 0.1961] Reset Explode Loop - Resets the exploded battlebot
  (if (< (`self.unexplodeDelta`) 1.0)
    (for (_array_element _array_index) (`self.explodeComponents`)
      (set `self.unexplodeDelta` _returnvalue)
      (`SceneComponent.K2_SetRelativeLocation` _array_element (`KismetMathLibrary.VLerp` (`|GetArrayItem` (`self.endVector`) _array_index) (`|GetArrayItem` (`self.baseVectors`) _array_index) _returnvalue) false false))))

(event `ResettingLoop`
  (`self.MoveTo`))

(event `self.ReceiveTick`
  (params (DeltaSeconds :type "Float (single-precision)"))
  ;[1 1 1] Main Handler
  (set `self.deltaSeconds` DeltaSeconds)
  (`|ExecutionSequence`
    (:`then_0`
      (if (not (`|EnumEquality` (`self.prevBattlebotState`) (`self.battlebotState`)))
        (`self.StateSwap`)
        (set `self.prevBattlebotState` (`self.battlebotState`))))
    (:`then_1`
      (if (not (`self.resetting`))
        (`self.BattlebotLoop`)
        (else
          (`self.ResettingLoop`))))))

(event `Reset State`
  ;[1 0.2039 0.1961] Resets all variables and transforms
  (set `self.resetting` true)
  (set `self.explodingTime` 0.0)
  (`|ExecutionSequence`
    (:`then_0`
      (switch `/Game/Battlebot/Blueprints/BattlebotState` (`self.battlebotState`)
        (:`NewEnumerator0`
          (set `self.degrees` 270.0))))
    (:`then_1`
      (`self.StopFollowPath`)
      (`self.ResetExplode`))))

(event `MoveTo`
  (bind _returnvalue (+ (* (`GameplayStatics.GetWorldDeltaSeconds`) 2.0) (`self.moveToDelta`)))
  (bind (_returnvalue_location _returnvalue_rotation) (`KismetMathLibrary.BreakTransform` (`KismetMathLibrary.TLerp` (`self.moveToStart`) (`self.moveToEnd`) _returnvalue)))
  ;[1 0.2039 0.1961] Move To - Animates the movement between states
  (if (< (`self.moveToDelta`) 1.0)
    (set `self.moveToDelta` _returnvalue)
    (`SceneComponent.K2_SetRelativeLocationAndRotation` (`self.BattleBot Mesh`) _returnvalue_location _returnvalue_rotation false false)
    (else
      (set `self.resetting` false))))

(event `BattlebotLoop`
  (bind _battlebotstate (`self.battlebotState`))
  ;[1 1 1] Movement Loop
  (`|ExecutionSequence`
    (:`then_0`
      (switch `/Game/Battlebot/Blueprints/BattlebotState` _battlebotstate
        (:`NewEnumerator0`
          (`self.Driving`))
        (:`NewEnumerator1`
          (`self.Hovering`))
        (:`NewEnumerator2`
          (`self.Explode`))))
    (:`then_1`
      (switch `/Game/Battlebot/Blueprints/BattlebotState` _battlebotstate
        (:`NewEnumerator0`
          _)
        (:`NewEnumerator1`
          _))
      (`self.ResetExplodeLoop`))))

(event `Driving`
  (`self.MoveWheels`)
  (`self.FollowPath`))

(event `FollowPath`
  (bind _road (`self.Road`))
  ;[0.2313 1 0.6485] Follow Path
  (`TimelineComponent.SetPlayRate` (`self.Timeline`) (/ 1.0 (`self.Time To Complete (In Seconds)`)))
  (bind (_direction _move_track) (`Timeline|Timeline` :!label _label_2)
    (:`Update`
      (bind _returnvalue (`KismetMathLibrary.Lerp` (`SplineComponent.GetSplineLength` (`self.Road`)) 0.0 _move_track))
      (`self.K2_SetActorTransform` (`KismetMathLibrary.MakeTransform` (`SplineComponent.GetLocationAtDistanceAlongSpline` _road _returnvalue "World") (`SplineComponent.GetRotationAtDistanceAlongSpline` _road _returnvalue "Local") (`self.GetActorScale3D`))))))

(event `StopFollowPath`
  ;[0.2313 1 0.6485] Follow Path
  (goto _label_2 :!via `Stop`))

(event `MoveWheels`
  ;[0.2313 1 0.6485] Move Wheels
  (for _array_element (`self.wheels`)
    (`SceneComponent.K2_AddLocalRotation` _array_element (`KismetMathLibrary.MakeRotator` 0.0 (* (`self.driveSpeed`) (`self.deltaSeconds`))) false false)))

(event `Hovering`
  (bind _deltaseconds (`self.deltaSeconds`))
  ;[0.2313 1 0.6485] Hovering
  (`self.K2_AddActorWorldRotation` (`KismetMathLibrary.MakeRotator` 0.0 0.0 (* _deltaseconds (`self.hoverRotationSpeed`))))
  (bind _output_get (set `self.degrees` (`KismetMathLibrary.FMod` (+ (`self.degrees`) (* _deltaseconds (`self.hoverSpeed`))) 360.0)))
  (`SceneComponent.K2_SetRelativeLocation` (`self.BattleBot Mesh`) (`KismetMathLibrary.MakeVector` 0.0 0.0 (* (`self.hoverHeight`) (+ (`KismetMathLibrary.DegSin` _output_get) 1.0))) false false))

(event `Explode`
  (bind _deltaseconds (`self.deltaSeconds`))
  ;[0.2313 1 0.6485] Exploding
  (if (> (`self.explodingDuration`) (`self.explodingTime`))
    (for (_array_element _array_index) (`self.explodeComponents`)
      (set `self.explodingTime` (+ _deltaseconds (`self.explodingTime`)))
      (bind _returnvalue_location (`KismetMathLibrary.BreakTransform` (`SceneComponent.GetRelativeTransform` _array_element)))
      (`SceneComponent.K2_SetRelativeLocation` _array_element (+ _returnvalue_location (* (* (`|GetArrayItem` (`self.moveVectors`) _array_index) (`self.explodeSpeed`)) _deltaseconds)) false false))))

(event `Spin`
  (params (rotation :type "Float (double-precision)"))
  ;[0.2313 1 0.6485] Handles dragging in explode mode
  (`SceneComponent.K2_AddRelativeRotation` (`self.BattleBot Mesh`) (`KismetMathLibrary.MakeRotator` 0.0 0.0 rotation) false false))

(fn `UserConstructionScript`)