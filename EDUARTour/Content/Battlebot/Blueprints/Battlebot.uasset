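; Battlebot Blueprint that spins its mesh and bobs it up and down as a hover animation.
; Tick accumulates an angle from RotationSpeed, wraps it at 360 for yaw, and feeds its sine, scaled by HoverHeight, into relative height, syncing bob with spin.
; The offset passes through the local transform of an empty, newly made AR trace result, not a real trace.
; An older world-transform location update remains disconnected.
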(event `self.ReceiveTick`
  (params (DeltaSeconds :type "Float (single-precision)"))
  (bind _output_get (set `self.rotation` (+ (* DeltaSeconds (`self.rotationSpeed`)) (`self.rotation`))))
  (bind _remainder (`KismetMathLibrary.FMod` _output_get 360.0))
  (`SceneComponent.K2_SetRelativeRotation` (`self.BattleBot Mesh`) (`KismetMathLibrary.MakeRotator` 0.0 180.0 _remainder) false false)
  (`SceneComponent.K2_SetRelativeLocation` (`self.BattleBot Mesh`) (`KismetMathLibrary.TransformLocation` (`ARTraceResultLibrary.GetLocalTransform` (make `ARTraceResult`)) (`KismetMathLibrary.MakeVector` 0.0 0.0 (* (`KismetMathLibrary.DegSin` _remainder) (`self.hoverHeight`)))) false false))

(fn `UserConstructionScript`)