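; ArrowStartBP is a guide arrow that points the player through an ordered list of Locations, apparently for an educational AR tour.
; Each tick it sits ahead of the camera at a fixed height, tilted and yawed toward the current location.
; When the camera's horizontal distance to that location drops below DistanceToHide, it advances the index, printing both values for debugging.
; After the last location, the arrow component is hidden.
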(event `self.ReceiveTick`
  (params (DeltaSeconds :type "Float (single-precision)"))
  (bind _returnvalue (`GameplayStatics.GetPlayerCameraManager` 0))
  (bind _returnvalue_2 (`PlayerCameraManager.GetCameraLocation` _returnvalue))
  (bind (_returnvalue_x _returnvalue_y) (`KismetMathLibrary.BreakVector` (- (`|GetArrayItem` (`self.locations`) (`self.currentLocation`)) _returnvalue_2)))
  (bind _returnvalue_3 (- (`|GetArrayItem` (`self.locations`) (`self.currentLocation`)) (`self.K2_GetActorLocation`)))
  (bind (_returnvalue_x_2 _returnvalue_y_2) (`KismetMathLibrary.BreakVector` (`KismetMathLibrary.TransformLocation` (`KismetMathLibrary.Conv_VectorToTransform` _returnvalue_2) (* (`self.GetActorForwardVector` _returnvalue) (300.0 300.0 0.0)))))
  (bind _returnvalue_4 (`KismetMathLibrary.VSize` (`KismetMathLibrary.MakeVector` _returnvalue_x _returnvalue_y -0.0)))
  (if (>= (`self.currentLocation`) (`KismetArrayLibrary.Array_Length` (`self.locations`)))
    (`SceneComponent.SetVisibility` (`self.ArrowEduArTour`) false false)
    (else
      (`self.K2_SetActorLocationAndRotation` (`KismetMathLibrary.MakeVector` _returnvalue_x_2 _returnvalue_y_2 -175.0) (`KismetMathLibrary.MakeRotator` 0.0 20.0 (.yaw (`KismetMathLibrary.MakeRotFromXY` _returnvalue_3 _returnvalue_3))))
      (`KismetSystemLibrary.PrintString` (`KismetStringLibrary.Conv_DoubleToString` _returnvalue_4))
      (if (< _returnvalue_4 (`self.distanceToHide`))
        (bind _output_get (set `self.currentLocation` (+ 1 (`self.currentLocation`))))
        (`KismetSystemLibrary.PrintString` (`KismetStringLibrary.Conv_IntToString` _output_get))))))

(fn `UserConstructionScript`)